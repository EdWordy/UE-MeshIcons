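; BP_MeshIconMaker is an editor utility actor that renders a static mesh into an icon texture asset.
; CreateIcon limits its scene capture to the actor's own components, resizes RT_MeshIconMaker to the set dimensions and assigns SourceMesh.
; It then captures the scene and saves the render target as a named static texture with icon compression, using an editor-only function.
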(event Custom|CreateIcon
  (Rendering|SceneCapture|ShowOnlyActorComponents (Variables|Default|GetSceneCaptureComponent2D) self false)
  (Rendering|ResizeRenderTarget2D "/MeshIcons/Assets/RT_MeshIconMaker.RT_MeshIconMaker" (Variables|Default|GetWidth) (Variables|Default|GetHeight))
  (Components|StaticMesh|SetStaticMesh (Variables|Default|GetStaticMesh) (Variables|Default|GetSourceMesh))
  (Rendering|SceneCapture|CaptureScene (Variables|Default|GetSceneCaptureComponent2D) :!class /Script/Engine.SceneCaptureComponent2D)
  (Class|KismetRenderingLibrary|RenderTargetCreateStaticTexture2DEditorOnly "/MeshIcons/Assets/RT_MeshIconMaker.RT_MeshIconMaker" (Variables|Default|GetName) "TC_EditorIcon" "TMGS_FromTextureGroup"))

(fn ConstructionScript)